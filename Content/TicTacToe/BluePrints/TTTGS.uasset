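; Tic-tac-toe game state that holds the tiles and both players' win counts and supplies AI moves.
; Victory checks test the eight lines, detect draws through a product of tile owners, update wins by player one's side and notify the TTTGM game mode.
; The AI picks random free tiles; medium difficulty prefers critical tiles completing either player's pair, found by hardcoded per-tile neighbor checks.
; It also pushes UI updates and toggles tile debug numbers.
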(event Custom|EventDrawDebug
  ;[1 1 1] Toggle drawDebug
  (for _array_element (Variables|Default|GetListTiles)
    (Default|EventToggleDebugNumbers _array_element)))

(event Custom|Event_CheckVictory
  (bind _returnvalue (Game|GetGameMode))
  (bind _p1side (Variables|Default|GetP1side))
  (bind _returnvalue_2 (== _p1side 1))
  (bind _astttgm (Utilities|Casting|CastToTTTGM _returnvalue))
  ;[1 1 1] Print Debug
  (bind _winner (CallFunction|CheckLines (Variables|Default|GetListTiles)))
  (switch int _winner
    (:-1
      (Default|EventGetDraw _astttgm))
    (:1
      (if _returnvalue_2
        (Math|Integer|IncrementInt (Variables|Default|GetP1wins) :!label _label
          (:%20%20
            (Default|EventGetVictory _astttgm 2)))
        (else
          (Math|Integer|IncrementInt (Variables|Default|GetP2wins) :!label _label_2
            (:%20%20
              (Default|EventGetVictory _astttgm 1))))))
    (:2
      (if _returnvalue_2
        (goto _label_2)
        (else
          (goto _label))))))

(event EventBeginPlay
  (Utilities|FlowControl|Delay 0.1)
  (CallFunction|UpdateButtonOwner))

(fn ConstructionScript)

(fn CheckLine
  (params (Array :type Array%20of%20TTT%20Tile%20Object%20References) (ID1 :type Integer) (ID2 :type Integer) (ID3 :type Integer))
  (bind _output (Utilities|Array|Get(acopy) Array ID3))
  (bind _output_2 (Utilities|Array|Get(acopy) Array ID2))
  (bind _playerid (Variables|/Game/TicTacToe/BluePrints/TTTTile.TTTTile_C|GetPlayerId _output))
  (bind _playerid_2 (Variables|/Game/TicTacToe/BluePrints/TTTTile.TTTTile_C|GetPlayerId _output_2))
  (if (Math|Boolean|ANDBoolean (== (Variables|/Game/TicTacToe/BluePrints/TTTTile.TTTTile_C|GetPlayerId (Utilities|Array|Get(acopy) Array ID1)) _playerid_2) (== _playerid_2 _playerid) (!= _playerid 0))
    (bind _output_get (Variables|Default|SetWinner _playerid)))
  (return _output_get))

(fn CheckLines
  (params (Array :type Array%20of%20TTT%20Tile%20Object%20References))
  (Variables|Default|SetWinner 0)
  (bind _winner (CallFunction|CheckLine Array 0 1 2))
  (if (Math|Conversions|ToBoolean(Integer) _winner)
    _
    (else
      (bind _winner_2 (CallFunction|CheckLine Array 3 4 5))
      (if (Math|Conversions|ToBoolean(Integer) _winner_2)
        _
        (else
          (bind _winner_3 (CallFunction|CheckLine Array 6 7 8))
          (if (Math|Conversions|ToBoolean(Integer) _winner_3)
            _
            (else
              (bind _winner_4 (CallFunction|CheckLine Array 0 3 6))
              (if (Math|Conversions|ToBoolean(Integer) _winner_4)
                _
                (else
                  (bind _winner_5 (CallFunction|CheckLine Array 1 4 7))
                  (if (Math|Conversions|ToBoolean(Integer) _winner_5)
                    _
                    (else
                      (bind _winner_6 (CallFunction|CheckLine Array 2 5 8))
                      (if (Math|Conversions|ToBoolean(Integer) _winner_6)
                        _
                        (else
                          (bind _winner_7 (CallFunction|CheckLine Array 0 4 8))
                          (if (Math|Conversions|ToBoolean(Integer) _winner_7)
                            _
                            (else
                              (bind _winner_8 (CallFunction|CheckLine Array 2 4 6))
                              (if (Math|Conversions|ToBoolean(Integer) _winner_8)
                                _
                                (else
                                  ;[1 1 1] Check for draw!
                                  (for _array_element Array
                                    (LocalVariables|Settemp_prod (* (Variables|/Game/TicTacToe/BluePrints/TTTTile.TTTTile_C|GetPlayerId _array_element) (LocalVariables|Gettemp_prod))))
                                  (if (!= (LocalVariables|Gettemp_prod) 0)
                                    (Variables|Default|SetWinner -1))))))))))))))))))
  (return (Variables|Default|GetWinner)))

(fn UpdateButtonOwner
  (Default|CallUpdateUI (Variables|Default|GetListTiles) (Variables|Default|GetP1wins) (Variables|Default|GetP2wins) (Variables|Default|GetP1side)))

(fn AIGetMove
  (params (Player%20Index :type Integer))
  (bind _possible (LocalVariables|Getpossible))
  (bind _possible_2 (LocalVariables|Getpossible))
  (bind _possible_3 (LocalVariables|Getpossible))
  (bind _ai_level (Variables|Default|GetAi_Level))
  (bind _returnvalue (Utilities|Array|Length _possible_2))
  (if (> (Variables|Default|GetAi_Level) 0)
    ;[1 1 1] get list of possible moves
    (Utilities|Array|Clear _possible)
    (for _array_element (Variables|Default|GetListTiles)
      (if (== (Variables|/Game/TicTacToe/BluePrints/TTTTile.TTTTile_C|GetPlayerId _array_element) 0)
        (Utilities|Array|Add _possible _array_element)))
    (Utilities|FlowControl|Sequence
      (:then_0
        ;[1 1 1] stop if no possible move
        (if (not (== _returnvalue 0))
          (Development|PrintString (Utilities|String|Append "Difficulty: " (Utilities|String|ToString(Integer) _ai_level)))
          (switch int _ai_level
            (:1
              ;[1 1 1] Easy AI: random move
              (LocalVariables|Setfounded true)
              (LocalVariables|SetplayTile (Utilities|Array|Get(acopy) (LocalVariables|Getpossible) (Math|Random|RandomInteger _returnvalue))))
            (:2
              ;[1 1 1] Medium AI: random move but try to win
              (LocalVariables|Setfounded true)
              (LocalVariables|SetplayTile (Utilities|Array|Get(acopy) _possible_3 (Math|Random|RandomInteger _returnvalue)))
              (bind _array_element_2 (Utilities|Array|ForEachLoopwithBreak _possible_3 :!label _label)
                (:LoopBody
                  (bind _critical (CallFunction|IsCritical (Variables|/Game/TicTacToe/BluePrints/TTTTile.TTTTile_C|GetId _array_element_2)))
                  (if _critical
                    (LocalVariables|SetplayTile _array_element_2)
                    (goto _label Break))))))))
      (:then_1
        (return (LocalVariables|Getfounded) (LocalVariables|GetplayTile) Player%20Index)))
    (else
      (return (LocalVariables|Getfounded) (LocalVariables|GetplayTile) Player%20Index))))

(fn IsCritical
  (params (Id :type Integer))
  (bind _playerid (Utilities|GetTilePID 6))
  (bind _playerid_2 (Utilities|GetTilePID 2))
  (bind _playerid_3 (Utilities|GetTilePID 4))
  (bind _playerid_4 (Utilities|GetTilePID 7))
  (bind _playerid_5 (Utilities|GetTilePID))
  (bind _playerid_6 (Utilities|GetTilePID 4))
  (bind _playerid_7 (Utilities|GetTilePID 6))
  (bind _playerid_8 (Utilities|GetTilePID 1))
  (bind _playerid_9 (Utilities|GetTilePID 1))
  (bind _playerid_10 (Utilities|GetTilePID 3))
  (bind _playerid_11 (Utilities|GetTilePID 4))
  (bind _playerid_12 (Utilities|GetTilePID 4))
  (bind _playerid_13 (Utilities|GetTilePID))
  (bind _playerid_14 (Utilities|GetTilePID 5))
  (bind _playerid_15 (Utilities|GetTilePID 4))
  (bind _playerid_16 (Utilities|GetTilePID))
  (bind _playerid_17 (Utilities|GetTilePID 4))
  (bind _playerid_18 (Utilities|GetTilePID 3))
  (bind _playerid_19 (Utilities|GetTilePID 1))
  (bind _playerid_20 (Utilities|GetTilePID))
  (bind _playerid_21 (Utilities|GetTilePID 3))
  (bind _playerid_22 (Utilities|GetTilePID 2))
  (bind _playerid_23 (Utilities|GetTilePID 2))
  (Utilities|FlowControl|Sequence
    (:then_0
      (switch int Id
        (:0
          ;[1 1 1] tile 0
          (LocalVariables|Setcrit (Math|Boolean|ORBoolean (and (!= _playerid_9 0) (== _playerid_9 (Utilities|GetTilePID 2))) (and (!= _playerid_10 0) (== _playerid_10 (Utilities|GetTilePID 2))) (and (!= _playerid_11 0) (== _playerid_11 (Utilities|GetTilePID 8))))))
        (:1
          ;[1 1 1] tile 1
          (LocalVariables|Setcrit (or (and (!= 0 0) (== (Utilities|GetTilePID) (Utilities|GetTilePID 2))) (and (!= _playerid_12 0) (== _playerid_12 (Utilities|GetTilePID 7))))))
        (:2
          ;[1 1 1] tile 2
          (LocalVariables|Setcrit (Math|Boolean|ORBoolean (and (!= _playerid_13 0) (== _playerid_13 (Utilities|GetTilePID 1))) (and (!= _playerid_14 0) (== _playerid_14 (Utilities|GetTilePID 8))) (and (!= _playerid_15 0) (== _playerid_15 (Utilities|GetTilePID 6))))))
        (:3
          ;[1 1 1] 3
          (LocalVariables|Setcrit (or (and (!= _playerid_16 0) (== _playerid_16 (Utilities|GetTilePID 6))) (and (!= _playerid_17 0) (== _playerid_17 (Utilities|GetTilePID 5))))))
        (:4
          ;[1 1 1] tile 4
          (LocalVariables|Setcrit (Math|Boolean|ORBoolean (and (!= _playerid_18 0) (== _playerid_18 (Utilities|GetTilePID 5))) (and (!= _playerid_19 0) (== _playerid_19 (Utilities|GetTilePID 7))) (and (!= _playerid_23 0) (== _playerid_23 (Utilities|GetTilePID 6))) (and (!= _playerid_20 0) (== _playerid_20 (Utilities|GetTilePID 8))))))
        (:5
          ;[1 1 1] tile 5
          (LocalVariables|Setcrit (or (and (!= _playerid_21 0) (== _playerid_21 (Utilities|GetTilePID 4))) (and (!= _playerid_22 0) (== _playerid_22 (Utilities|GetTilePID 8))))))
        (:6
          ;[1 1 1] tile 6
          (LocalVariables|Setcrit (Math|Boolean|ORBoolean (and (!= _playerid_4 0) (== _playerid_4 (Utilities|GetTilePID 8))) (and (!= _playerid_5 0) (== _playerid_5 (Utilities|GetTilePID 3))) (and (!= _playerid_6 0) (== _playerid_6 (Utilities|GetTilePID 2))))))
        (:7
          ;[1 1 1] tile 7
          (LocalVariables|Setcrit (or (and (!= _playerid_7 0) (== _playerid_7 (Utilities|GetTilePID 8))) (and (!= _playerid_8 0) (== _playerid_8 (Utilities|GetTilePID 4))))))
        (:8
          ;[1 1 1] tile 8
          (LocalVariables|Setcrit (Math|Boolean|ORBoolean (and (!= _playerid 0) (== _playerid (Utilities|GetTilePID 7))) (and (!= _playerid_2 0) (== _playerid_2 (Utilities|GetTilePID 5))) (and (!= _playerid_3 0) (== _playerid_3 (Utilities|GetTilePID))))))))
    (:then_1
      (return (LocalVariables|Getcrit)))))