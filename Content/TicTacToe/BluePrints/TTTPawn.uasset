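; Player pawn for a Tic-Tac-Toe game that holds the nine tile child actors and handles all board input.
; Each tick it traces from the cursor to highlight the pointed tile.
; A touch drag spins the base plate with torque through a gate, while a release under the drag threshold claims the tile and switches player.
; It also registers tiles with the game state, resets the board, and handles debug and menu keys.
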(event Custom|EventREsetBorad
  (bind _returnvalue (Game|GetGameState))
  (bind _astttgs (Utilities|Casting|CastToTTTGS _returnvalue))
  ;[1 1 1] reset the board
  (Variables|/Game/TicTacToe/BluePrints/TTTGS.TTTGS_C|SetP1side _astttgs (+ (Math|Integer|%(Integer) (Variables|/Game/TicTacToe/BluePrints/TTTGS.TTTGS_C|GetP1side _astttgs) 2) 1))
  (for _array_element (Variables|Default|GetButtonList)
    (Default|EventChangeOwner _array_element)
    (Default|EventGotoGame (.AsTTTGM (Utilities|Casting|CastToTTTGM (Game|GetGameMode))))))

(event EventTick
  (params (DeltaSeconds :type Float%20%28single-precision%29))
  (bind _returnvalue (Pawn|GetController))
  (bind _mouseposition (Variables|Default|GetmousePosition))
  (bind _astttpc (Utilities|Casting|CastToTTTPC _returnvalue))
  (bind (_locationx _locationy) (Game|Player|GetMousePosition _astttpc))
  (bind _returnvalue_2 (Math|Vector|MakeVector _locationx _locationy 0.0))
  (bind _returnvalue_3 (- _returnvalue_2 _mouseposition))
  (bind (_x _y) (Math|Vector|BreakVector _returnvalue_3))
  (Utilities|FlowControl|Sequence
    (:then_0
      ;[1 1 1] Reset hightlighted property
      (if (not (Game|IsGamePaused))
        (for _array_element (Variables|Default|GetButtonList)
          (Default|EventChangeHightligh _array_element false))
        (Utilities|CalcMouseWorldPos
          (:NewParam2
            (bind _asttttile (Utilities|GetPointedTile)
              (:then
                (Default|EventChangeHightligh _asttttile true)))))))
    (:then_1
      ;[1 1 1] baseplate movement
      (Utilities|FlowControl|Gate true
        (:Exit
          (Class|PrimitiveComponent|AddTorqueinRadians (Variables|Default|GetbasePlate) (* (Math|Vector|MakeVector 0.0 _y (* _x -1.0)) (Variables|Default|GetRotationSpeed)) "None" false))))))

(event Input|KeyboardEvents|D
  (params (Key :type Key%20Structure))
  ;[1 1 1] Debug informations
  (:Pressed
    (bind _astttgs (Utilities|Casting|CastToTTTGS (Game|GetGameState)))
    (Default|EventDrawDebug _astttgs)))

(event Input|KeyboardEvents|Escape
  (params (Key :type Key%20Structure))
  ;[1 1 1] Return To main Menu
  (:Pressed
    (if (not (Game|IsGamePaused))
      (Default|EventGotoMainMenu (.AsTTTGM (Utilities|Casting|CastToTTTGM (Game|GetGameMode)))))))

(event Input|TouchEvents|InputTouch
  (params (Location :type Vector) (FingerIndex :type ETouchIndex%20Enum))
  (bind _returnvalue (Pawn|GetController))
  (bind _returnvalue_2 (Game|GetGameState))
  (bind _mouseposition (Variables|Default|GetmousePosition))
  (bind _astttpc (Utilities|Casting|CastToTTTPC _returnvalue))
  (bind _astttgs (Utilities|Casting|CastToTTTGS _returnvalue_2))
  (bind (_locationx _locationy) (Game|Player|GetMousePosition _astttpc))
  (bind _returnvalue_3 (Math|Vector|MakeVector _locationx _locationy 0.0))
  (bind _returnvalue_4 (- _returnvalue_3 _mouseposition))
  (bind (_x _y) (Math|Vector|BreakVector _returnvalue_4))
  (:Pressed
    (Variables|Default|SetMousePosition _returnvalue_3)
    ;[1 1 1] baseplate movement
    (Utilities|FlowControl|Gate true) ; enters at Open
  )
  (:Released
    (if (< (Math|Vector|VectorLength _returnvalue_4) (Variables|Default|GetDragThreshold))
      (Utilities|FlowControl|Sequence
        (:then_0
          ;[1 1 1] play on tile
          (bind _asttttile (Utilities|GetPointedTile)
            (:then
              (Default|EventChangeOwner _asttttile (Variables|/Game/TicTacToe/BluePrints/TTTGS.TTTGS_C|GetCurrentPalyer _astttgs))
              (Variables|/Game/TicTacToe/BluePrints/TTTGS.TTTGS_C|SetCurrentPalyer _astttgs (+ (Math|Integer|%(Integer) (Variables|/Game/TicTacToe/BluePrints/TTTGS.TTTGS_C|GetCurrentPalyer _astttgs) 2) 1)))))
        (:then_1
          (Utilities|FlowControl|Gate true) ; enters at Close
        ))
      (else
        (Utilities|FlowControl|Gate true) ; enters at Close
      ))))

(fn ConstructionScript
  (bind _buttonlist (Variables|Default|GetButtonList))
  (for (_array_element _array_index) (Utilities|Array|MakeArray (Variables|Default|GetButton_11) (Variables|Default|GetButton_12) (Variables|Default|GetButton_13) (Variables|Default|GetButton_21) (Variables|Default|GetButton_22) (Variables|Default|GetButton_23) (Variables|Default|GetButton_31) (Variables|Default|GetButton_32) (Variables|Default|GetButton_33))
    (Variables|/Game/TicTacToe/BluePrints/TTTTile.TTTTile_C|SetId (.AsTTTTile (Utilities|Casting|CastToTTTTile (Variables|/Script/Engine.ChildActorComponent|GetChildActor _array_element))) _array_index)
    (Utilities|Array|AddUnique _buttonlist (.AsTTTTile (Utilities|Casting|CastToTTTTile (Variables|/Script/Engine.ChildActorComponent|GetChildActor _array_element)))))
  (Variables|/Game/TicTacToe/BluePrints/TTTGS.TTTGS_C|SetListTiles (.AsTTTGS (Utilities|Casting|CastToTTTGS (Game|GetGameState))) _buttonlist))