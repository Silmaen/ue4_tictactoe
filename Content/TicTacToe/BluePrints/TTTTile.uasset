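; Tic-tac-toe board tile that shows its owner as an empty button, cross or round.
; An owner change, gated by a pause or zero-PlayerId check, swaps mesh and material, then tells TTTGS to update button ownership.
; Highlighting drives the State parameter of a dynamic material created at BeginPlay, only while the tile is unowned.
; A toggleable gate on Tick draws the tile Id as debug text.
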(event Custom|EventChangeOwner
  (params (PlayerId :type Integer))
  (bind _button (Variables|Default|Getbutton))
  ;[1 1 1] Change tIle Owner
  (if (or (Game|IsGamePaused) (== (Variables|Default|GetPlayerId) 0))
    (bind _output_get (Variables|Default|SetPlayerId PlayerId))
    (if (== _output_get 0)
      (Components|StaticMesh|SetStaticMesh _button "/Game/TicTacToe/Meshes/button.button")
      (Rendering|Material|SetMaterial _button 0 "/Game/TicTacToe/Materials/ButtonMaterial.ButtonMaterial")
      (elif (== _output_get 1)
        (Components|StaticMesh|SetStaticMesh _button "/Game/TicTacToe/Meshes/cross.cross")
        (Rendering|Material|SetMaterial _button 0 "/Game/TicTacToe/Materials/CrossMaterial.CrossMaterial")
        (else
          (Components|StaticMesh|SetStaticMesh _button "/Game/TicTacToe/Meshes/round.round")
          (Rendering|Material|SetMaterial _button 0 "/Game/TicTacToe/Materials/RoundMaterial.RoundMaterial"))))
    (Default|UpdateButtonOwner (.AsTTTGS (Utilities|Casting|CastToTTTGS (Game|GetGameState))))))

(event Custom|EventChangeHightligh
  (params (HightLighted :type Boolean))
  (bind _dynamat (Variables|Default|GetDynaMat))
  ;[1 1 1] hight light the button
  (bind _output_get (Variables|Default|SetHightLighted HightLighted))
  (if (== 0 (Variables|Default|GetPlayerId))
    (if _output_get
      (Rendering|Material|SetScalarParameterValue _dynamat "State" 1.0 :!class /Script/Engine.MaterialInstanceDynamic)
      (else
        (Rendering|Material|SetScalarParameterValue _dynamat "State" 0.0 :!class /Script/Engine.MaterialInstanceDynamic)))))

(event Custom|EventToggleDebugNumbers
  ;[1 1 1] Print Debug
  (Utilities|FlowControl|Gate true) ; enters at Toggle
)

(event EventBeginPlay
  (bind _button (Variables|Default|Getbutton))
  ;[1 1 1] Initialize
  (bind _returnvalue (Rendering|Material|CreateDynamicMaterialInstance _button 0 "/Game/TicTacToe/Materials/ButtonMaterial.ButtonMaterial" "None" :!class /Script/Engine.PrimitiveComponent))
  (bind _output_get (Variables|Default|SetDynaMat _returnvalue))
  (Rendering|Material|SetMaterial _button 0 _output_get))

(event EventTick
  (params (DeltaSeconds :type Float%20%28single-precision%29))
  ;[1 1 1] Print Debug
  (Utilities|FlowControl|Gate true
    (:Exit
      (Rendering|Debug|DrawDebugString (Physics|GetCenterOfMass (Variables|Default|Getbutton) "None") (Utilities|String|ToString(Integer) (Variables|Default|GetId)) 0 "(R=1.000000,G=1.000000,B=1.000000,A=1.000000)"))))

(fn ConstructionScript)