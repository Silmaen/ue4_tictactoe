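; Tic-tac-toe game manager that owns the UI screens and switches between menus, gameplay and match results.
; BeginPlay creates menu and result widgets, shows only the main menu, then pauses with UI-only input after a short delay.
; Custom events toggle widget visibility, pause state and input mode per screen; victory shows Loser for WinnerId 1, otherwise Winner.
; WidgetGameHUD is toggled but never created here.
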(event Custom|EventGotoGame
  ;[1 1 1] Activate Game
  (Utilities|FlowControl|Sequence
    (:then_0
      (Widget|SetVisibility (Variables|Default|GetWidgetMainMenu) "Hidden"))
    (:then_1
      (Widget|SetVisibility (Variables|Default|GetWidgetOptionsMenu) "Hidden"))
    (:then_2
      (Widget|SetVisibility (Variables|Default|GetWidgetGameHUD) "Visible"))
    (:then_3
      (Widget|SetVisibility (Variables|Default|GetWidgetDraw) "Hidden"))
    (:then_4
      (Widget|SetVisibility (Variables|Default|GetWidgetLoser) "Hidden"))
    (:then_5
      (Widget|SetVisibility (Variables|Default|GetWidgetWinner) "Hidden"))
    (:then_6
      (Game|SetGamePaused false))
    (:then_7
      (Input|SetInputModeGameOnly (Game|GetPlayerController 0)))))

(event Custom|EventGotoOption
  ;[1 1 1] Activate Options Menu
  (Utilities|FlowControl|Sequence
    (:then_0
      (Widget|SetVisibility (Variables|Default|GetWidgetMainMenu) "Hidden"))
    (:then_1
      (Widget|SetVisibility (Variables|Default|GetWidgetOptionsMenu) "Visible"))
    (:then_2
      (Widget|SetVisibility (Variables|Default|GetWidgetGameHUD) "Hidden"))
    (:then_3
      (Widget|SetVisibility (Variables|Default|GetWidgetDraw) "Hidden"))
    (:then_4
      (Widget|SetVisibility (Variables|Default|GetWidgetLoser) "Hidden"))
    (:then_5
      (Widget|SetVisibility (Variables|Default|GetWidgetWinner) "Hidden"))
    (:then_6
      (Game|SetGamePaused true))
    (:then_7
      (Input|SetInputModeUIOnly (Game|GetPlayerController 0) 0 "DoNotLock"))))

(event Custom|EventGotoMainMenu
  ;[1 1 1] Activate Main Menu
  (Utilities|FlowControl|Sequence
    (:then_0
      (Widget|SetVisibility (Variables|Default|GetWidgetMainMenu) "Visible"))
    (:then_1
      (Widget|SetVisibility (Variables|Default|GetWidgetOptionsMenu) "Hidden"))
    (:then_2
      (Widget|SetVisibility (Variables|Default|GetWidgetGameHUD) "Hidden"))
    (:then_3
      (Widget|SetVisibility (Variables|Default|GetWidgetDraw) "Hidden"))
    (:then_4
      (Widget|SetVisibility (Variables|Default|GetWidgetLoser) "Hidden"))
    (:then_5
      (Widget|SetVisibility (Variables|Default|GetWidgetWinner) "Hidden"))
    (:then_6
      (Game|SetGamePaused true))
    (:then_7
      (Input|SetInputModeUIOnly (Game|GetPlayerController 0) 0 "DoNotLock"))))

(event Custom|EventGetVictory
  (params (WinnerId :type Integer))
  (bind _returnvalue (== WinnerId 1))
  ;[1 1 1] Activate Main Menu
  (Utilities|FlowControl|Sequence
    (:then_0
      (Widget|SetVisibility (Variables|Default|GetWidgetMainMenu) "Hidden"))
    (:then_1
      (Widget|SetVisibility (Variables|Default|GetWidgetOptionsMenu) "Hidden"))
    (:then_2
      (Widget|SetVisibility (Variables|Default|GetWidgetGameHUD) "Hidden"))
    (:then_3
      (Widget|SetVisibility (Variables|Default|GetWidgetDraw) "Hidden"))
    (:then_4
      (Widget|SetVisibility (Variables|Default|GetWidgetLoser) (select _returnvalue "Visible" "Hidden")))
    (:then_5
      (Widget|SetVisibility (Variables|Default|GetWidgetWinner) (select _returnvalue "Hidden" "Visible")))
    (:then_6
      (Game|SetGamePaused true))
    (:then_7
      (Input|SetInputModeUIOnly (Game|GetPlayerController 0) 0 "DoNotLock"))))

(event Custom|EventGetDraw
  ;[1 1 1] Activate Main Menu
  (Utilities|FlowControl|Sequence
    (:then_0
      (Widget|SetVisibility (Variables|Default|GetWidgetMainMenu) "Hidden"))
    (:then_1
      (Widget|SetVisibility (Variables|Default|GetWidgetOptionsMenu) "Hidden"))
    (:then_2
      (Widget|SetVisibility (Variables|Default|GetWidgetGameHUD) "Hidden"))
    (:then_3
      (Widget|SetVisibility (Variables|Default|GetWidgetDraw) "Visible"))
    (:then_4
      (Widget|SetVisibility (Variables|Default|GetWidgetLoser) "Hidden"))
    (:then_5
      (Widget|SetVisibility (Variables|Default|GetWidgetWinner) "Hidden"))
    (:then_6
      (Game|SetGamePaused true))
    (:then_7
      (Input|SetInputModeUIOnly (Game|GetPlayerController 0) 0 "DoNotLock"))))

(event EventBeginPlay
  (bind _returnvalue (Game|GetPlayerController 0))
  ;[1 1 1] Creation and Initialization of the Widgets
  (Utilities|FlowControl|Sequence
    (:then_0
      (bind _returnvalue_2 (UserInterface|CreateWidget "/Game/TicTacToe/BluePrints/Menu/MainMenu.MainMenu_C" _returnvalue))
      (bind _output_get (Variables|Default|SetWidgetMainMenu _returnvalue_2))
      (UserInterface|Viewport|AddtoViewport _output_get 0)
      (Widget|SetVisibility _output_get "Visible"))
    (:then_1
      (bind _returnvalue_3 (UserInterface|CreateWidget "/Game/TicTacToe/BluePrints/Menu/OptionsMenu.OptionsMenu_C" _returnvalue))
      (bind _output_get_2 (Variables|Default|SetWidgetOptionsMenu _returnvalue_3))
      (UserInterface|Viewport|AddtoViewport _output_get_2 0)
      (Widget|SetVisibility _output_get_2 "Hidden"))
    (:then_2
      (Utilities|FlowControl|Delay 0.2)
      (Game|SetGamePaused true)
      (Input|SetInputModeUIOnly _returnvalue 0 "DoNotLock"))
    (:then_3
      (bind _returnvalue_4 (UserInterface|CreateWidget "/Game/TicTacToe/BluePrints/HUD/Draw.Draw_C" _returnvalue))
      (bind _output_get_3 (Variables|Default|SetWidgetDraw _returnvalue_4))
      (UserInterface|Viewport|AddtoViewport _output_get_3 0)
      (Widget|SetVisibility _output_get_3 "Hidden"))
    (:then_4
      (bind _returnvalue_5 (UserInterface|CreateWidget "/Game/TicTacToe/BluePrints/HUD/Loser.Loser_C" _returnvalue))
      (bind _output_get_4 (Variables|Default|SetWidgetLoser _returnvalue_5))
      (UserInterface|Viewport|AddtoViewport _output_get_4 0)
      (Widget|SetVisibility _output_get_4 "Hidden"))
    (:then_5
      (bind _returnvalue_6 (UserInterface|CreateWidget "/Game/TicTacToe/BluePrints/HUD/Winner.Winner_C"))
      (bind _output_get_5 (Variables|Default|SetWidgetWinner _returnvalue_6))
      (UserInterface|Viewport|AddtoViewport _output_get_5 0)
      (Widget|SetVisibility _output_get_5 "Hidden"))))

(fn ConstructionScript)